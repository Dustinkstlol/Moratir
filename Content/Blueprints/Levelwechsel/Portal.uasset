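; Level-change portal actor that lets the player travel to another level by pressing E inside its trigger.
; Overlap by Moratir_BP enables input and shows a Dialogue_Widget with the portal's text; leaving disables input and removes the widget.
; Pressing E stores the DoorID in MyGameInstance and calls its smooth level load, using the Destination enum converted to a level name.
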(event OnComponentBeginOverlap(PortalTrigger)
  (params (OverlappedComponent :type Primitive%20Component%20Object%20Reference) (OtherActor :type Actor%20Object%20Reference) (OtherComp :type Primitive%20Component%20Object%20Reference) (OtherBodyIndex :type Integer) (bFromSweep :type Boolean) (SweepResult :type Hit%20Result%20Structure%20%28by%20ref%29))
  (bind _returnvalue (Game|GetPlayerController 0))
  (Utilities|Casting|CastToMoratir_BP OtherActor)
  (Input|EnableInput _returnvalue)
  (bind _returnvalue_2 (UserInterface|CreateWidget "/Game/Blueprints/NPC/Inanimate/Dialogue_Widget.Dialogue_Widget_C" _returnvalue))
  (bind _output_get (Variables|Default|SetDialogueWidgetz _returnvalue_2))
  (UserInterface|Viewport|AddtoViewport _output_get 0)
  (Variables|/Game/Blueprints/NPC/Inanimate/Dialogue_Widget.Dialogue_Widget_C|SetDialogueText (Variables|Default|GetDialogueWidgetz) (Variables|Default|GetText)))

(event OnComponentEndOverlap(PortalTrigger)
  (params (OverlappedComponent :type Primitive%20Component%20Object%20Reference) (OtherActor :type Actor%20Object%20Reference) (OtherComp :type Primitive%20Component%20Object%20Reference) (OtherBodyIndex :type Integer))
  (Utilities|Casting|CastToMoratir_BP OtherActor)
  (Input|DisableInput (Game|GetPlayerController 0))
  (Widget|RemovefromParent (Variables|Default|GetDialogueWidgetz))
  (Variables|Default|SetDialogueWidgetz 0))

(event Input|KeyboardEvents|E
  (params (Key :type Key%20Structure :default "None"))
  (:Pressed
    (bind _asmy_game_instance (Utilities|Casting|CastToMyGameInstance (Game|GetGameInstance)))
    (Variables|/Game/Blueprints/Levelwechsel/MyGameInstance.MyGameInstance_C|SetDoorID _asmy_game_instance (Variables|Default|GetDoorID))
    (Default|EventSmoothLoadLevel _asmy_game_instance (Utilities|String|StringToName (Utilities|String|EnumtoString (Variables|Default|GetDestination))))))

(fn ConstructionScript)