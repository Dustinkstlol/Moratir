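; Puppenhaus_BP is an inanimate interactable that shows up to three timed lines of text.
; It creates a Text_Widget on BeginPlay and enables player input when Moratir_BP overlaps its box.
; Depending on SpielAutomatisch, the text plays once automatically on overlap or each time Interact fires.
; A delay of the summed text durations plus one second then removes the widget.
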(event OnComponentBeginOverlap(Box)
  (params (OverlappedComponent :type Primitive%20Component%20Object%20Reference) (OtherActor :type Actor%20Object%20Reference) (OtherComp :type Primitive%20Component%20Object%20Reference) (OtherBodyIndex :type Integer) (bFromSweep :type Boolean) (SweepResult :type Hit%20Result%20Structure%20%28by%20ref%29))
  (bind _textwidget (Variables|Default|GetTextWidget))
  (Utilities|Casting|CastToMoratir_BP OtherActor)
  (Input|EnableInput (Game|GetPlayerController 0))
  (if (Variables|Default|GetSpielAutomatisch?)
    (if (not (Variables|Default|GetSchonGespielt))
      (Variables|Default|SetSchonGespielt true)
      (UserInterface|Viewport|AddtoViewport (Variables|Default|GetTextWidget) 0)
      (Utilities|FlowControl|Sequence
        (:then_0
          (Default|Begin _textwidget (Variables|Default|GetMyText1) (Variables|Default|GetMyText2) (Variables|Default|GetMyText3))
          (Variables|/Game/Blueprints/NPC/Inanimate/Text_Widget.Text_Widget_C|Set2 _textwidget (Variables|Default|Get2texte?))
          (Variables|/Game/Blueprints/NPC/Inanimate/Text_Widget.Text_Widget_C|Set3 _textwidget (Variables|Default|Get3Texte?))
          (Variables|/Game/Blueprints/NPC/Inanimate/Text_Widget.Text_Widget_C|SetTextdauer1 _textwidget (Variables|Default|Getlenght1))
          (Variables|/Game/Blueprints/NPC/Inanimate/Text_Widget.Text_Widget_C|SetTextdauer2 _textwidget (Variables|Default|Getlenght2))
          (Variables|/Game/Blueprints/NPC/Inanimate/Text_Widget.Text_Widget_C|SetTextdauer3 _textwidget (Variables|Default|Getlenght3)))
        (:then_1
          (Utilities|FlowControl|Delay (+ (Variables|Default|Getlenght1) (Variables|Default|Getlenght2) (Variables|Default|Getlenght3) 1.0))
          (CallFunction|EndChat))))))

(event OnComponentEndOverlap(Box)
  (params (OverlappedComponent :type Primitive%20Component%20Object%20Reference) (OtherActor :type Actor%20Object%20Reference) (OtherComp :type Primitive%20Component%20Object%20Reference) (OtherBodyIndex :type Integer)))

(event Custom|EndChat
  (Widget|RemovefromParent (Variables|Default|GetTextWidget)))

(event EventBeginPlay
  (bind _returnvalue (UserInterface|CreateWidget "/Game/Blueprints/NPC/Inanimate/Text_Widget.Text_Widget_C"))
  (bind _output_get (Variables|Default|SetTextWidget _returnvalue))
  (Variables|/Game/Blueprints/NPC/Inanimate/Text_Widget.Text_Widget_C|SetTriggerRef _output_get self))

(event EventInteract
  (bind _textwidget (Variables|Default|GetTextWidget))
  (if (not (Variables|Default|GetSpielAutomatisch?))
    (UserInterface|Viewport|AddtoViewport (Variables|Default|GetTextWidget) 0)
    (Utilities|FlowControl|Sequence
      (:then_0
        (Default|Begin _textwidget (Variables|Default|GetMyText1) (Variables|Default|GetMyText2) (Variables|Default|GetMyText3))
        (Variables|/Game/Blueprints/NPC/Inanimate/Text_Widget.Text_Widget_C|Set2 _textwidget (Variables|Default|Get2texte?))
        (Variables|/Game/Blueprints/NPC/Inanimate/Text_Widget.Text_Widget_C|Set3 _textwidget (Variables|Default|Get3Texte?))
        (Variables|/Game/Blueprints/NPC/Inanimate/Text_Widget.Text_Widget_C|SetTextdauer1 _textwidget (Variables|Default|Getlenght1))
        (Variables|/Game/Blueprints/NPC/Inanimate/Text_Widget.Text_Widget_C|SetTextdauer2 _textwidget (Variables|Default|Getlenght2))
        (Variables|/Game/Blueprints/NPC/Inanimate/Text_Widget.Text_Widget_C|SetTextdauer3 _textwidget (Variables|Default|Getlenght3)))
      (:then_1
        (Utilities|FlowControl|Delay (+ (Variables|Default|Getlenght1) (Variables|Default|Getlenght2) (Variables|Default|Getlenght3) 1.0))
        (CallFunction|EndChat)))))

(fn ConstructionScript)