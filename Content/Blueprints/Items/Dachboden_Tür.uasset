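; Attic door actor that swaps a wall mesh for a door when switched.
; The Switch function calls WandSwap, which sets IsOpen, plays a grinding door sound at world origin, destroys WandMesh and makes TürMesh visible.
; TürMesh is also made visible on BeginPlay, and the swap has no reverse path because the wall component is destroyed.
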(event Custom|WandSwap
  (Variables|Default|SetisOpen true)
  (Audio|PlaySoundatLocation "/Game/Audio/Events/Door_Grinding_open.Door_Grinding_open" "0, 0, 0" "0, 0, 0" 1.0 1.0 0.0 0 0 0)
  (Components|DestroyComponent (Variables|Default|GetWandMesh))
  (Rendering|SetVisibility (Variables|Default|GetTürMesh) true false))

(event EventBeginPlay
  (Rendering|SetVisibility (Variables|Default|GetTürMesh) true false))

(fn ConstructionScript)

(fn Switch
  (CallFunction|WandSwap))