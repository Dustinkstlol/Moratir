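; Armor actor that reacts to a linked ArmorSchalter_BP switch, apparently meant to move aside.
; Switch calls HebeGitter ("lift grate"), which plays Beiseite ("aside") only if the SwitchActor reports IsOpen.
; The BeginPlay check of the switch does nothing, and the SetRelativeLocation nodes on ArmorMesh are unconnected, so this graph never moves the mesh.
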(event Custom|HebeGitter
  (bind _asarmor_schalter_bp (Utilities|Casting|CastToArmorSchalter_BP (Variables|Default|GetSwitchActor)))
  (if (Variables|/Game/Blueprints/Items/ArmorSchalter_BP.ArmorSchalter_BP_C|GetIsOpen _asarmor_schalter_bp)
    (Timeline|Beiseite! Play)))

(event EventBeginPlay
  (bind _asarmor_schalter_bp (Utilities|Casting|CastToArmorSchalter_BP (Variables|Default|GetSwitchActor)))
  (if (Variables|/Game/Blueprints/Items/ArmorSchalter_BP.ArmorSchalter_BP_C|GetIsOpen _asarmor_schalter_bp)
    _))

(fn ConstructionScript)

(fn Switch
  (CallFunction|HebeGitter))