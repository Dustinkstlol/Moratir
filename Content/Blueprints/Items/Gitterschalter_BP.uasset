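; Gitterschalter_BP is a lever switch that operates the Gitter_BP grate actors in the level.
; Its box trigger enables input and shows a text prompt while a Moratir_BP overlaps it.
; Pressing E flips IsOpen and plays the Spin timeline, which yaws the Hebel lever.
; Every timeline update also calls Switch on all Gitter_BP actors, so that call repeats throughout playback.
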(event OnComponentBeginOverlap(Box)
  (params (OverlappedComponent :type Primitive%20Component%20Object%20Reference) (OtherActor :type Actor%20Object%20Reference) (OtherComp :type Primitive%20Component%20Object%20Reference) (OtherBodyIndex :type Integer) (bFromSweep :type Boolean) (SweepResult :type Hit%20Result%20Structure%20%28by%20ref%29))
  (Utilities|Casting|CastToMoratir_BP OtherActor)
  (Input|EnableInput (Game|GetPlayerController 0))
  (Rendering|SetVisibility (Variables|Default|GetTextRender) true false))

(event OnComponentEndOverlap(Box)
  (params (OverlappedComponent :type Primitive%20Component%20Object%20Reference) (OtherActor :type Actor%20Object%20Reference) (OtherComp :type Primitive%20Component%20Object%20Reference) (OtherBodyIndex :type Integer))
  (Utilities|Casting|CastToMoratir_BP OtherActor)
  (Input|DisableInput (Game|GetPlayerController 0))
  (Rendering|SetVisibility (Variables|Default|GetTextRender) false false))

(event Input|KeyboardEvents|E
  (params (Key :type Key%20Structure))
  (:Pressed
    (Variables|Default|SetIsOpen (not (Variables|Default|GetIsOpen)))
    (bind _spin (Timeline|Spin Play)
      (:Update
        (Transformation|SetRelativeRotation (Variables|Default|GetHebel) (Math|Rotator|MakeRotator 0.0 0.0 _spin) false false)
        (bind _outactors (Actor|GetAllActorsOfClass "/Game/Blueprints/Items/Gitter_BP.Gitter_BP_C"))
        (for _array_element _outactors
          (Default|Switch _array_element))))))

(fn ConstructionScript)