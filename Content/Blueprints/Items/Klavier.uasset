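; Klavier is an interactable piano for a quest to collect black piano keys, responding to Moratir_BP through a dialogue widget.
; A box overlap toggles input and a text prompt, while Interact opens or closes the dialogue, showing intro text on first use.
; Later uses scan the inventory for a full key stack, then either play a delayed piano sound or show searching text.
; Leaving the actor's overlap closes the dialogue, and MusikSpielen is an empty stub.
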(event OnComponentBeginOverlap(Box)
  (params (OverlappedComponent :type Primitive%20Component%20Object%20Reference) (OtherActor :type Actor%20Object%20Reference) (OtherComp :type Primitive%20Component%20Object%20Reference) (OtherBodyIndex :type Integer) (bFromSweep :type Boolean) (SweepResult :type Hit%20Result%20Structure%20%28by%20ref%29))
  ;[1 1 1] Lass Moratir mit E interagieren
  (Utilities|Casting|CastToMoratir_BP OtherActor)
  (Input|EnableInput (Game|GetPlayerController 0))
  (Rendering|SetVisibility (Variables|Default|GetTextRender) true false))

(event OnComponentEndOverlap(Box)
  (params (OverlappedComponent :type Primitive%20Component%20Object%20Reference) (OtherActor :type Actor%20Object%20Reference) (OtherComp :type Primitive%20Component%20Object%20Reference) (OtherBodyIndex :type Integer))
  ;[1 1 1] Lass Moratir mit E interagieren
  (Utilities|Casting|CastToMoratir_BP OtherActor)
  (Input|DisableInput (Game|GetPlayerController 0))
  (Rendering|SetVisibility (Variables|Default|GetTextRender) false false))

(event Custom|Weitersuchen
  (Development|PrintString "Ich muss wohl noch weiteruschen")
  (Variables|/Game/Blueprints/NPC/Variant1/Dialogue_Widget.Dialogue_Widget_C|SetDialogueText (Variables|Default|GetDialogueWidget) (Variables|Texte|GetNoch%20nicht%20genug)))

(event Custom|Key1%20eingesetzt
  (Development|PrintString "Key1 ist da")
  (Variables|/Game/Blueprints/NPC/Variant1/Dialogue_Widget.Dialogue_Widget_C|SetDialogueText (Variables|Default|GetDialogueWidget) (Variables|Texte|GetErsterKey))
  (Utilities|FlowControl|Delay 2.0)
  (Audio|PlaySoundatLocation "/Game/Audio/Events/Piano_Test_Loop.Piano_Test_Loop" "0, 0, 0" "0, 0, 0" 1.0 1.0 0.0 0 0 0))

(event Custom|MusikSpielen)

(event Collision|EventActorEndOverlap
  (params (OtherActor :type Actor%20Object%20Reference))
  ;[1 1 1] Schließe das Widget wenn Spieler weggeht
  (Utilities|IsValid (Variables|Default|GetDialogueWidget)
    (:Is%20Valid
      (Widget|RemovefromParent (Variables|Default|GetDialogueWidget))
      (Variables|Default|SetDialogueWidget 0))))

(event EventInteract
  ;[1 1 1] Erstelle das Widdget
  (Utilities|IsValid (Variables|Default|GetDialogueWidget)
    (:Is%20Valid
      (Widget|RemovefromParent (Variables|Default|GetDialogueWidget))
      (Variables|Default|SetDialogueWidget 0))
    (:Is%20Not%20Valid
      (bind _returnvalue (UserInterface|CreateWidget "/Game/Blueprints/NPC/Variant1/Dialogue_Widget.Dialogue_Widget_C" (Game|GetPlayerController 0)))
      (bind _output_get (Variables|Default|SetDialogueWidget _returnvalue))
      (UserInterface|Viewport|AddtoViewport _output_get 0)
      (if (Variables|Default|GetFirstInteraction?)
        (Variables|/Game/Blueprints/NPC/Variant1/Dialogue_Widget.Dialogue_Widget_C|SetDialogueText (Variables|Default|GetDialogueWidget) (Variables|Texte|GetStartText))
        (Variables|Default|SetFirstInteraction? false)
        (else
          (CallFunction|CheckforKeys))))))

(fn ConstructionScript)

(fn CheckforKeys
  (bind _asmoratir_bp (Utilities|Casting|CastToMoratir_BP (Game|GetPlayerCharacter 0)))
  (bind _array_element (Utilities|Array|ForEachLoopwithBreak (Variables|/Game/Blueprints/Inventar/UI/Inventory.Inventory_C|GetInventorySlotArray (Variables|/Game/Charaktere/Moratir/Blueprints/Moratir_BP.Moratir_BP_C|GetInventoryWidget _asmoratir_bp)) :!label _label)
    (:LoopBody
      (if (Utilities|Enum|Equal(Enum) (.name (Variables|/Game/Blueprints/Inventar/UI/InventorySlot.InventorySlot_C|GetItem%20Info _array_element)) "Black Piano Key")
        (if (== (.sizestackid (Variables|/Game/Blueprints/Inventar/UI/InventorySlot.InventorySlot_C|GetItem%20Info _array_element)) 3)
          (Variables|Default|SetAlleKeysinBesitz? true)
          (goto _label Break)
          (else
            (Variables|Default|SetMoreKeysMissing true)
            (goto _label Break)))
        (else
          (Variables|/Game/Blueprints/NPC/Variant1/Dialogue_Widget.Dialogue_Widget_C|SetDialogueText (Variables|Default|GetDialogueWidget) (Variables|Texte|GetBeginSearch)))))
    (:Completed
      (if (Variables|Default|GetAlleKeysinBesitz?)
        (CallFunction|Key1Eingesetzt)
        (elif (Variables|Default|GetMoreKeysMissing)
          (CallFunction|Weitersuchen))))))