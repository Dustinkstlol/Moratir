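; Library armor pedestal item that switches from showing its pedestal mesh to showing an armor mesh when triggered.
; On BeginPlay the pedestal (PodestMesh) is visible and the armor (RüstungMesh) is hidden.
; The Switch function calls the HebeGitter ("raise grate") event, which reverses both visibilities without propagating to children.
; The swap is one-way and moves nothing, despite the event's name.
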(event Custom|HebeGitter
  (Rendering|SetVisibility (Variables|Default|GetRüstungMesh) true false)
  (Rendering|SetVisibility (Variables|Default|GetPodestMesh) false false))

(event EventBeginPlay
  (Rendering|SetVisibility (Variables|Default|GetRüstungMesh) false false)
  (Rendering|SetVisibility (Variables|Default|GetPodestMesh) true false))

(fn ConstructionScript)

(fn Switch
  (CallFunction|HebeGitter))