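; Gitter_BP is a grate whose mesh slides when its linked Gitterschalter_BP switch is open.
; Its Switch function calls HebeGitter, which checks the IsOpen state on SwitchActor and plays a timeline that drives the mesh's relative location.
; BeginPlay runs the same check with a separate timeline, so a switch that is already open moves the grate at start.
; The file contains no reverse or closing path.
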(event Custom|HebeGitter
  (bind _asgitterschalter_bp (Utilities|Casting|CastToGitterschalter_BP (Variables|Default|GetSwitchActor)))
  (if (Variables|/Game/Blueprints/Items/Gitterschalter_BP.Gitterschalter_BP_C|GetIsOpen _asgitterschalter_bp)
    (bind _gitterslide (Timeline|Timeline_0 Play)
      (:Update
        (Transformation|SetRelativeLocation (Variables|Default|GetGitterMesh) _gitterslide false false)))))

(event EventBeginPlay
  (bind _asgitterschalter_bp (Utilities|Casting|CastToGitterschalter_BP (Variables|Default|GetSwitchActor)))
  (if (Variables|/Game/Blueprints/Items/Gitterschalter_BP.Gitterschalter_BP_C|GetIsOpen _asgitterschalter_bp)
    (bind _gitterslide (Timeline|GitterAnim Play)
      (:Update
        (Transformation|SetRelativeLocation (Variables|Default|GetGitterMesh) _gitterslide false false)))))

(fn ConstructionScript)

(fn Switch
  (CallFunction|HebeGitter))