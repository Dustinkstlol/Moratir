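; MusikControl_BP is a trigger-box actor that switches an ambient music sound when Moratir_BP enters.
; On BeginPlay it caches whether music is allowed from the Klavier reference's BackgroundAllowed, defaulting to true without one.
; Entry while off fades music in if allowed.
; Entry while on passes through a FlipFlop, alternating between fading out and repeating the fade-in, so not every such entry stops playback.
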(event OnComponentBeginOverlap(Box)
  (params (OverlappedComponent :type Primitive%20Component%20Object%20Reference) (OtherActor :type Actor%20Object%20Reference) (OtherComp :type Primitive%20Component%20Object%20Reference) (OtherBodyIndex :type Integer) (bFromSweep :type Boolean) (SweepResult :type Hit%20Result%20Structure%20%28by%20ref%29))
  (bind _ambientsound (Variables|Default|GetAmbientSound))
  (bind _audiocomponent (Variables|/Script/Engine.AmbientSound|GetAudioComponent _ambientsound))
  (Utilities|Casting|CastToMoratir_BP OtherActor)
  (if (Variables|Default|GetIstSchonAn?)
    (Utilities|FlowControl|FlipFlop
      (:A
        (Audio|Components|Audio|FadeOut _audiocomponent 3.0 0.0 "Linear" :!class /Script/Engine.AudioComponent)
        (Variables|Default|SetIstSchonAn? false))
      (:B
        (if (Variables|Default|GetDarfMusikAn?) :!label _label
          (Audio|Components|Audio|FadeIn _audiocomponent 3.0 (Variables|Default|GetMaxVolume) 0.0 "Linear" :!class /Script/Engine.AudioComponent)
          (Variables|Default|SetIstSchonAn? true))))
    (else
      (goto _label))))

(event EventBeginPlay
  (bind _klavier (Variables|Default|GetKlavier))
  (Utilities|IsValid _klavier
    (:Is%20Valid
      (Variables|Default|SetDarfMusikAn? (Variables|/Game/Blueprints/Items/Klavier.Klavier_C|GetBackgroundAllowed? _klavier)))
    (:Is%20Not%20Valid
      (Variables|Default|SetDarfMusikAn? true))))

(fn ConstructionScript)