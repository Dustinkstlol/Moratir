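; Cellar door Blueprint (Kellertür) that lets the player open a pivoting wall piece with E.
; A box trigger enables input while Moratir_BP overlaps it and disables it on exit.
; E plays the Einrasten timeline, which moves WandPivot's relative location.
; A two-second Delay on that timeline's Update output then starts the Drehung timeline, which rotates the pivot around its roll axis.
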(event OnComponentBeginOverlap(BoxTrigger)
  (params (OverlappedComponent :type Primitive%20Component%20Object%20Reference) (OtherActor :type Actor%20Object%20Reference) (OtherComp :type Primitive%20Component%20Object%20Reference) (OtherBodyIndex :type Integer) (bFromSweep :type Boolean) (SweepResult :type Hit%20Result%20Structure%20%28by%20ref%29))
  (Utilities|Casting|CastToMoratir_BP OtherActor)
  (Input|EnableInput (Game|GetPlayerController 0)))

(event OnComponentEndOverlap(BoxTrigger)
  (params (OverlappedComponent :type Primitive%20Component%20Object%20Reference) (OtherActor :type Actor%20Object%20Reference) (OtherComp :type Primitive%20Component%20Object%20Reference) (OtherBodyIndex :type Integer))
  (Utilities|Casting|CastToMoratir_BP OtherActor)
  (Input|DisableInput (Game|GetPlayerController 0)))

(event Input|KeyboardEvents|E
  (params (Key :type Key%20Structure :default "None"))
  (:Pressed
    (bind _down (Timeline|Einrasten Play)
      (:Update
        (Transformation|SetRelativeLocation (Variables|Default|GetWandPivot) _down false false)
        (Utilities|FlowControl|Delay 2.0)
        (bind _spin (Timeline|Drehung Play)
          (:Update
            (Transformation|SetRelativeRotation (Variables|Default|GetWandPivot) (Math|Rotator|MakeRotator _spin 0.0 0.0) false false)))))))

(fn ConstructionScript)