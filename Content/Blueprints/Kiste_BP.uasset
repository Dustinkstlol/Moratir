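; Kiste_BP is a chest that the player character, Moratir_BP, opens by pressing E while inside its trigger box.
; Overlapping the box enables input on the chest and shows a text prompt if it is still closed; leaving disables input and hides the prompt.
; E plays the Drehung timeline, which rolls ChestPivot by its Spin track, hides the prompt and sets IsOpen.
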(event OnComponentBeginOverlap(BoxTrigger)
  (params (OverlappedComponent :type Primitive%20Component%20Object%20Reference) (OtherActor :type Actor%20Object%20Reference) (OtherComp :type Primitive%20Component%20Object%20Reference) (OtherBodyIndex :type Integer) (bFromSweep :type Boolean) (SweepResult :type Hit%20Result%20Structure%20%28by%20ref%29))
  (Utilities|Casting|CastToMoratir_BP OtherActor)
  (Input|EnableInput (Game|GetPlayerController 0))
  (if (not (Variables|Default|GetIsOpen))
    (Rendering|SetVisibility (Variables|Default|GetTextRender) true false)))

(event OnComponentEndOverlap(BoxTrigger)
  (params (OverlappedComponent :type Primitive%20Component%20Object%20Reference) (OtherActor :type Actor%20Object%20Reference) (OtherComp :type Primitive%20Component%20Object%20Reference) (OtherBodyIndex :type Integer))
  (Utilities|Casting|CastToMoratir_BP OtherActor)
  (Input|DisableInput (Game|GetPlayerController 0))
  (Rendering|SetVisibility (Variables|Default|GetTextRender) false false))

(event Input|KeyboardEvents|E
  (params (Key :type Key%20Structure :default "None"))
  (:Pressed
    (bind _spin (Timeline|Drehung Play)
      (:Update
        (Transformation|SetRelativeRotation (Variables|Default|GetChestPivot) (Math|Rotator|MakeRotator _spin 0.0 0.0) false false)
        (Rendering|SetVisibility (Variables|Default|GetTextRender) false false)
        (Variables|Default|SetIsOpen true)))))

(fn ConstructionScript)