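; Checkpoint actor with a box trigger that removes itself at level start if the save game already records it as used.
; BeginPlay loads the "save1" slot as BP_Savegame and destroys the actor if its CheckpointUsed collection contains this instance.
; Box overlap repeats the load and lookup but does nothing with the result, so this Blueprint never records or saves a checkpoint.
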(event OnComponentBeginOverlap(Box)
  (params (OverlappedComponent :type Primitive%20Component%20Object%20Reference) (OtherActor :type Actor%20Object%20Reference) (OtherComp :type Primitive%20Component%20Object%20Reference) (OtherBodyIndex :type Integer) (bFromSweep :type Boolean) (SweepResult :type Hit%20Result%20Structure%20%28by%20ref%29))
  (bind _returnvalue (SaveGame|LoadGamefromSlot "save1"))
  (bind _asbp_savegame (Utilities|Casting|CastToBP_Savegame _returnvalue))
  (if (Utilities|Array|ContainsItem (Variables|/Game/Blueprints/Saving/BP_Savegame.BP_Savegame_C|GetCheckpointUsed _asbp_savegame) self)
    _))

(event EventBeginPlay
  (bind _returnvalue (SaveGame|LoadGamefromSlot "save1"))
  (bind _asbp_savegame (Utilities|Casting|CastToBP_Savegame _returnvalue))
  (if (Utilities|Array|ContainsItem (Variables|/Game/Blueprints/Saving/BP_Savegame.BP_Savegame_C|GetCheckpointUsed _asbp_savegame) self)
    (Actor|DestroyActor)))

(fn ConstructionScript)