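; Special one-off door that plays a house cutscene when interacted with.
; Overlapping the front trigger caches Moratir and enables input on that character; leaving disables input on the door itself.
; Interact destroys the door object, plays the video through a VideoWidget, reveals the referenced Krippe mesh and teleports Moratir along negative Y.
; It also stores a facing check in Richtung, which nothing here reads.
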(event OnComponentBeginOverlap(Vorderseite)
  (params (OverlappedComponent :type Primitive%20Component%20Object%20Reference) (OtherActor :type Actor%20Object%20Reference) (OtherComp :type Primitive%20Component%20Object%20Reference) (OtherBodyIndex :type Integer) (bFromSweep :type Boolean) (SweepResult :type Hit%20Result%20Structure%20%28by%20ref%29))
  (bind _asmoratir_bp (Utilities|Casting|CastToMoratir_BP OtherActor))
  (Variables|Default|SetMoratirRef _asmoratir_bp)
  (Input|EnableInput _asmoratir_bp (Game|GetPlayerController 0)))

(event OnComponentEndOverlap(Vorderseite)
  (params (OverlappedComponent :type Primitive%20Component%20Object%20Reference) (OtherActor :type Actor%20Object%20Reference) (OtherComp :type Primitive%20Component%20Object%20Reference) (OtherBodyIndex :type Integer))
  (Utilities|Casting|CastToMoratir_BP OtherActor)
  (Input|DisableInput (Game|GetPlayerController 0)))

(event EventInteract
  (bind _moratirref (Variables|Default|GetMoratirRef))
  (bind _returnvalue (Transformation|GetActorLocation _moratirref))
  (Variables|Default|SetRichtung (Math|Vector|Equal(Vector) (Transformation|GetActorForwardVector) (Math|Vector|Normalize (- (Transformation|GetActorLocation (Game|GetPlayerController 0)) (Transformation|GetActorLocation))) 1.0))
  (Components|DestroyComponent (Variables|Default|Getobj_Einzeltür))
  (bind _returnvalue_2 (UserInterface|CreateWidget "/Game/Cinematics/Sequences/FilmAbspielen/VideoWidget.VideoWidget_C"))
  (UserInterface|Viewport|AddtoViewport _returnvalue_2 0)
  (Default|PlayVideo _returnvalue_2 (Utilities|Struct|MakeFilmStructure "/Game/Cinematics/Sequences/FilmAbspielen/NewMediaPlayer_Video_Mat.NewMediaPlayer_Video_Mat" "/Game/Movies/Moratir_Cutscenes.Moratir_Cutscenes" "/Game/Cinematics/Sequences/FilmAbspielen/DerWahreMediaPlayer.DerWahreMediaPlayer" "/Game/Cinematics/Sequences/FilmAbspielen/Haus_Cutscene.Haus_Cutscene"))
  (Rendering|SetVisibility (Variables|/Script/Engine.StaticMeshActor|GetStaticMeshComponent (Variables|Default|GetKrippe_Ref)) true false)
  (Transformation|SetWorldLocation (Variables|/Script/Engine.Actor|GetRootComponent _moratirref) (Math|Vector|MakeVector (.x _returnvalue) (- (.y _returnvalue) 4e+02) (.z _returnvalue)) false true))

(fn ConstructionScript)