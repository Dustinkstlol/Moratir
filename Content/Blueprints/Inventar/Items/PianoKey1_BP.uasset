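; PianoKey1_BP is an inventory pickup, named as a piano key, that spins in the world until collected.
; Interact casts the player character to Moratir_BP, adds ItemInfo to its InventoryWidget and destroys the actor.
; Tick yaws the root by DeltaSeconds plus one degree each frame, so spin speed depends on frame rate.
; UseItem is only a placeholder that prints a debug string.
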(event EventTick
  (params (DeltaSeconds :type Float%20%28single-precision%29))
  (Transformation|AddLocalRotation (Variables|Default|GetDefaultSceneRoot) (Math|Rotator|MakeRotator 0.0 0.0 (+ DeltaSeconds 1.0)) false false))

(event EventInteract
  (bind _asmoratir_bp (Utilities|Casting|CastToMoratir_BP (Game|GetPlayerCharacter 0)))
  (Default|AddtoInventory (Variables|/Game/Charaktere/Moratir/Blueprints/Moratir_BP.Moratir_BP_C|GetInventoryWidget _asmoratir_bp) (Variables|Default|GetItem_Info))
  (Actor|DestroyActor))

(event EventUseItem
  (Development|PrintString "UseItem1"))

(fn ConstructionScript
  (|CallParentFunction))