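; MoratirGamemode is a game mode that picks the player's spawn point from a door ID stored in the game instance.
; Its ChoosePlayerStart reads DoorID from MyGameInstance and returns the PlayerStart whose PlayerStartTag matches it.
; Without a match, it falls back to the first PlayerStart found in the level.
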(fn ConstructionScript)

(fn ChoosePlayerStart
  (params (Player :type Controller%20Object%20Reference))
  (bind _asmy_game_instance (Utilities|Casting|CastToMyGameInstance (Game|GetGameInstance)))
  (bind _outactors (Actor|GetAllActorsOfClass "/Script/Engine.PlayerStart"))
  (for _array_element _outactors
    (if (Utilities|Name|Equal(Name) (Variables|/Script/Engine.PlayerStart|GetPlayerStartTag _array_element) (Variables|/Game/Blueprints/Levelwechsel/MyGameInstance.MyGameInstance_C|GetDoorID _asmy_game_instance))
      (return _array_element)))
  (return (Utilities|Array|Get(acopy) _outactors)))