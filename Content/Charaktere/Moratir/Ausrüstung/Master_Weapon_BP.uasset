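; Base weapon Blueprint for the player character Moratir, handling combo attack montages and damage to enemies.
; Light and heavy attacks step through three- and two-stage chains stored on the character, flag the last attack and call empty combo events.
; HitEvent matches the hit actor against all Master_Enemy_BP actors, damaging unrecorded enemies, with a 30% heavy-attack bonus.
; AttackTrace is empty here, and the impact particle spawn is unconnected.
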(event Custom|LightAttack
  (bind _characterref (Variables|Default|GetCharacterRef))
  (bind _characterref_2 (Variables|Default|GetCharacterRef))
  (bind _characterref_3 (Variables|Default|GetCharacterRef))
  ;[1 1 1] Light Attack Animation
  (if (== (+ (Variables|/Game/Charaktere/Moratir/Blueprints/Moratir_BP.Moratir_BP_C|GetChainLight (Variables|Default|GetCharacterRef)) 1) (Utilities|Array|Length (Variables|Default|GetLightAttacks)))
    (Variables|/Game/Charaktere/Moratir/Blueprints/Moratir_BP.Moratir_BP_C|SetLastAttack _characterref true))
  (switch int (Variables|/Game/Charaktere/Moratir/Blueprints/Moratir_BP.Moratir_BP_C|GetChainLight _characterref)
    (:0
      (Animation|PlayAnimMontage _characterref_2 (Utilities|Array|Get(acopy) (Variables|Default|GetLightAttacks) (Variables|/Game/Charaktere/Moratir/Blueprints/Moratir_BP.Moratir_BP_C|GetChainLight _characterref_2)) 1.0 "None")
      (CallFunction|ComboLightAttack (Variables|/Game/Charaktere/Moratir/Blueprints/Moratir_BP.Moratir_BP_C|GetChainLight (Variables|Default|GetCharacterRef)))
      (Variables|/Game/Charaktere/Moratir/Blueprints/Moratir_BP.Moratir_BP_C|SetChainLight _characterref_3 1))
    (:1
      (Animation|PlayAnimMontage _characterref_2 (Utilities|Array|Get(acopy) (Variables|Default|GetLightAttacks) (Variables|/Game/Charaktere/Moratir/Blueprints/Moratir_BP.Moratir_BP_C|GetChainLight _characterref_2)) 1.0 "None")
      (CallFunction|ComboLightAttack (Variables|/Game/Charaktere/Moratir/Blueprints/Moratir_BP.Moratir_BP_C|GetChainLight (Variables|Default|GetCharacterRef)))
      (Variables|/Game/Charaktere/Moratir/Blueprints/Moratir_BP.Moratir_BP_C|SetChainLight _characterref_3 2))
    (:2
      (Animation|PlayAnimMontage _characterref_2 (Utilities|Array|Get(acopy) (Variables|Default|GetLightAttacks) (Variables|/Game/Charaktere/Moratir/Blueprints/Moratir_BP.Moratir_BP_C|GetChainLight _characterref_2)) 1.0 "None")
      (CallFunction|ComboLightAttack (Variables|/Game/Charaktere/Moratir/Blueprints/Moratir_BP.Moratir_BP_C|GetChainLight (Variables|Default|GetCharacterRef)))
      (Variables|/Game/Charaktere/Moratir/Blueprints/Moratir_BP.Moratir_BP_C|SetChainLight _characterref_3 0))))

(event Custom|Heavy%20Attack
  (bind _characterref (Variables|Default|GetCharacterRef))
  (bind _characterref_2 (Variables|Default|GetCharacterRef))
  (bind _characterref_3 (Variables|Default|GetCharacterRef))
  ;[1 1 1] Heavy Animation
  (if (== (+ (Variables|/Game/Charaktere/Moratir/Blueprints/Moratir_BP.Moratir_BP_C|GetChainHeavy (Variables|Default|GetCharacterRef)) 1) (Utilities|Array|Length (Variables|Default|GetHeavyAttacks)))
    (Variables|/Game/Charaktere/Moratir/Blueprints/Moratir_BP.Moratir_BP_C|SetLastAttack _characterref true))
  (switch int (Variables|/Game/Charaktere/Moratir/Blueprints/Moratir_BP.Moratir_BP_C|GetChainHeavy _characterref)
    (:0
      (Animation|PlayAnimMontage _characterref_2 (Utilities|Array|Get(acopy) (Variables|Default|GetHeavyAttacks) (Variables|/Game/Charaktere/Moratir/Blueprints/Moratir_BP.Moratir_BP_C|GetChainHeavy _characterref_2)) 1.0 "None")
      (CallFunction|ComboHeavyAttack (Variables|/Game/Charaktere/Moratir/Blueprints/Moratir_BP.Moratir_BP_C|GetChainHeavy (Variables|Default|GetCharacterRef)))
      (Variables|/Game/Charaktere/Moratir/Blueprints/Moratir_BP.Moratir_BP_C|SetChainHeavy _characterref_3 1))
    (:1
      (Animation|PlayAnimMontage _characterref_2 (Utilities|Array|Get(acopy) (Variables|Default|GetHeavyAttacks) (Variables|/Game/Charaktere/Moratir/Blueprints/Moratir_BP.Moratir_BP_C|GetChainHeavy _characterref_2)) 1.0 "None")
      (CallFunction|ComboHeavyAttack (Variables|/Game/Charaktere/Moratir/Blueprints/Moratir_BP.Moratir_BP_C|GetChainHeavy (Variables|Default|GetCharacterRef)))
      (Variables|/Game/Charaktere/Moratir/Blueprints/Moratir_BP.Moratir_BP_C|SetChainHeavy _characterref_3 0))))

(event Custom|ComboHeavyAttack
  (params (ChainHeavy :type Integer))
  ;[1 1 1] Heavy Animation
)

(event Custom|ComboLightAttack
  (params (ChainLight :type Integer))
  ;[1 1 1] Light Attack Animation
)

(event Custom|HitEvent
  (params (Damge :type Integer) (Hit :type Hit%20Result%20Structure))
  (bind _characterref (Variables|Default|GetCharacterRef))
  (Variables|Default|SetDamage Damge)
  (bind _outactors (Actor|GetAllActorsOfClass "/Game/Charaktere/Enemy/Master_Enemy_BP.Master_Enemy_BP_C"))
  (for _array_element _outactors
    (Variables|Default|SetDamagedEnemy _array_element)
    (if (and (== _array_element (.HitActor (Collision|BreakHitResult Hit))) (not (Utilities|Array|ContainsItem (Variables|Default|GetAlreadyDamagedEnemy) (Variables|Default|GetDamagedEnemy))))
      (Utilities|Array|Add (Variables|Default|GetAlreadyDamagedEnemy) (Variables|Default|GetDamagedEnemy))
      (if (Variables|/Game/Charaktere/Moratir/Blueprints/Moratir_BP.Moratir_BP_C|GetLightAttack _characterref)
        (Default|DealingDamage (Variables|Default|GetDamagedEnemy) (Variables|Default|GetDamage) (Variables|Default|GetCharacterRef))
        (elif (Variables|/Game/Charaktere/Moratir/Blueprints/Moratir_BP.Moratir_BP_C|GetHeavyAttack _characterref)
          (Default|DealingDamage (Variables|Default|GetDamagedEnemy) (+ (Variables|Default|GetDamage) (Math|Float|Truncate (* (Variables|Default|GetDamage) 0.3))) (Variables|Default|GetCharacterRef)))))))

(event EventBeginPlay
  ;[1 1 1] Moratir Refenerence
  (bind _asmoratir_bp (Utilities|Casting|CastToMoratir_BP (Game|GetPlayerCharacter 0)))
  (Variables|Default|SetCharacterRef _asmoratir_bp))

(fn ConstructionScript)

(fn AttackTrace)