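; Ghoul enemy Blueprint that tracks health, shows it on a health bar widget and plays an attack montage.
; DealingDamage subtracts from CurrentHealth, refreshes the bar and sets IsDamaged once health differs from MaxHealth.
; UpdateHealth casts the EnemyHealth component's widget to Enemy_health and sets its fill percent.
; The bar is hidden at BeginPlay and revealed only when health is not at maximum.
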(event Custom|Attack
  (Animation|Montage|PlayMontage (Variables|Character|GetMesh) 0))

(event EventBeginPlay
  ;[1 1 1] Hp Bar
  (Rendering|SetVisibility (Variables|Default|GetEnemyHealth) false false)
  (CallFunction|UpdateHealth))

(event EventDealingDamage
  (params (Damage :type Integer) (Sender :type Actor%20Object%20Reference))
  ;[1 1 1] Hp Bar
  (Variables|Default|SetCurrentHealth (- (Variables|Default|GetCurrentHealth) Damage))
  (CallFunction|UpdateHealth)
  (if (!= (Variables|Default|GetCurrentHealth) (Variables|Default|GetMaxHealth))
    (Variables|Default|SetIsDamaged true)))

(fn ConstructionScript)

(fn UpdateHealth
  (bind _asenemy_health (Utilities|Casting|CastToEnemy_health (UserInterface|GetUserWidgetObject (Variables|Default|GetEnemyHealth))))
  (Progress|SetPercent (Variables|/Game/Charaktere/Enemy/Enemy_health.Enemy_health_C|GetHealth _asenemy_health) (/ (Math|Conversions|ToFloat(Integer) (Variables|Default|GetCurrentHealth)) (Math|Conversions|ToFloat(Integer) (Variables|Default|GetMaxHealth))))
  (if (!= (Variables|Default|GetCurrentHealth) (Variables|Default|GetMaxHealth))
    (Rendering|SetVisibility (Variables|Default|GetEnemyHealth) true false))
  (return))