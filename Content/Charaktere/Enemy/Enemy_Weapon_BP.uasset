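; Enemy weapon Blueprint that applies damage to Moratir_BP actors it hits.
; HitEvent stores the damage, finds every Moratir_BP and damages the one matching the hit actor, passing EnemyRef as sender.
; An AlreadyDamagedPlayer list blocks repeat damage and is never cleared here.
; EnemyRef comes from casting player pawn 0 to Master_Enemy_BP on BeginPlay, and AttackTrace is empty.
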(event Custom|HitEvent
  (params (Damge :type Integer) (Hit :type Hit%20Result%20Structure))
  (Variables|Default|SetDamage Damge)
  (bind _outactors (Actor|GetAllActorsOfClass "/Game/Charaktere/Moratir/Blueprints/Moratir_BP.Moratir_BP_C"))
  (for _array_element _outactors
    (Variables|Default|SetDamagedPlayer _array_element)
    (if (and (== _array_element (.HitActor (Collision|BreakHitResult Hit))) (not (Utilities|Array|ContainsItem (Variables|Default|GetAlreadyDamagedPlayer) (Variables|Default|GetDamagedPlayer))))
      (Utilities|Array|Add (Variables|Default|GetAlreadyDamagedPlayer) (Variables|Default|GetDamagedPlayer))
      (Default|TakeDamage (Variables|Default|GetDamagedPlayer) (Variables|Default|GetDamage) (Variables|Default|GetEnemyRef)))))

(event EventBeginPlay
  ;[1 1 1] Moratir Refenerence
  (bind _asmaster_enemy_bp (Utilities|Casting|CastToMaster_Enemy_BP (Game|Player|GetPlayerPawn 0)))
  (Variables|Default|SetEnemyRef _asmaster_enemy_bp))

(fn ConstructionScript)

(fn AttackTrace)