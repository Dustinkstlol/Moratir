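; Interactive wall or stand torch holder that the player can light or extinguish with the E key.
; A box overlap with Moratir_BP enables input on the actor and shows a text prompt, and leaving reverses both.
; E flips IsOn and SwitchLight applies it to two point lights and the fire particles, as BeginPlay does initially.
; Extinguishing triggers a smoke puff and a smoke pillar that stops after a delay.
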(event OnComponentBeginOverlap(Box)
  (params (OverlappedComponent :type Primitive%20Component%20Object%20Reference) (OtherActor :type Actor%20Object%20Reference) (OtherComp :type Primitive%20Component%20Object%20Reference) (OtherBodyIndex :type Integer) (bFromSweep :type Boolean) (SweepResult :type Hit%20Result%20Structure%20%28by%20ref%29))
  ;[1 1 1] Wenn in Reichweite, ermöglicht Input und zeigt Rendertext
  (Utilities|Casting|CastToMoratir_BP OtherActor)
  (Input|EnableInput (Game|GetPlayerController 0))
  (Rendering|SetVisibility (Variables|Default|GetTextRender) true false))

(event OnComponentEndOverlap(Box)
  (params (OverlappedComponent :type Primitive%20Component%20Object%20Reference) (OtherActor :type Actor%20Object%20Reference) (OtherComp :type Primitive%20Component%20Object%20Reference) (OtherBodyIndex :type Integer))
  ;[1 1 1] Wenn in Reichweite, ermöglicht Input und zeigt Rendertext
  (Utilities|Casting|CastToMoratir_BP OtherActor)
  (Input|DisableInput (Game|GetPlayerController 0))
  (Rendering|SetVisibility (Variables|Default|GetTextRender) false false))

(event EventBeginPlay
  (bind _ison (Variables|Default|GetIsOn))
  ;[1 1 1] Schaltet Licht ein/aus
  (Rendering|SetVisibility (Variables|Default|GetPointLight) _ison false)
  (Rendering|SetVisibility (Variables|Default|GetPointLight1) _ison false)
  (Rendering|SetVisibility (Variables|Default|Get1_TorchFire_pt) _ison false))

(event Input|KeyboardEvents|E
  (params (Key :type Key%20Structure :default "None"))
  ;[1 1 1] Schaltet Lightswitch, aktiviert Rauch
  (:Pressed
    (Variables|Default|SetIsOn (not (Variables|Default|GetIsOn)))
    (CallFunction|SwitchLight)
    (if (Variables|Default|GetIsOn)
      (Components|Activation|Deactivate (Variables|Default|GetP_SmokePillar1))
      (else
        (Components|Activation|Activate (Variables|Default|GetP_SmokePuff2c) false)
        (Components|Activation|Activate (Variables|Default|GetP_SmokePillar1) false)
        (Utilities|FlowControl|Delay 5.0)
        (Components|Activation|Deactivate (Variables|Default|GetP_SmokePillar1))))))

(fn ConstructionScript)

(fn SwitchLight
  (bind _ison (Variables|Default|GetIsOn))
  (Rendering|SetVisibility (Variables|Default|GetPointLight) _ison false)
  (Rendering|SetVisibility (Variables|Default|GetPointLight1) _ison false)
  (Rendering|SetVisibility (Variables|Default|Get1_TorchFire_pt) _ison false))